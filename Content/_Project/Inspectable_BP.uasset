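; Inspectable object Blueprint that the player can pick up for a close look and later put back.
; On interact, it registers itself as the FirstPersonCharacter's InteractingActor, saves its root transform, snaps to the character's InspectPosition and disables the character's movement.
; Ending the interaction restores the saved transform, but this Blueprint does not re-enable movement.
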(event EventOnInteract
  (params (InteractingActor :type Actor%20Object%20Reference))
  ;[1 1 1] Set players interacting actor to me
  (bind _asfirst_person_character (Utilities|Casting|CastToFirstPersonCharacter InteractingActor))
  (Variables|/Game/FirstPersonBP/Blueprints/FirstPersonCharacter.FirstPersonCharacter_C|SetInteractingActor _asfirst_person_character self)
  ;[1 1 1] Set Original Position
  (Variables|Default|SetoriginalPosition (Transformation|GetWorldTransform (Variables|Default|GetDefaultSceneRoot)))
  ;[1 1 1] Set Inspect Positioin
  (Transformation|SetWorldTransform (Variables|Default|GetDefaultSceneRoot) (Transformation|GetWorldTransform (Variables|/Game/FirstPersonBP/Blueprints/FirstPersonCharacter.FirstPersonCharacter_C|GetInspect_Position _asfirst_person_character)) false false)
  (Pawn|Components|CharacterMovement|SetMovementMode (Variables|/Script/Engine.Character|GetCharacterMovement _asfirst_person_character) "MOVE_None" 0))

(event EventOnEndInteraction
  ;[1 1 1] Set back to original position
  (Transformation|SetWorldTransform (Variables|Default|GetDefaultSceneRoot) (Variables|Default|GetoriginalPosition) false false))

(fn ConstructionScript)